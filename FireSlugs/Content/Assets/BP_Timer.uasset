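; BP_Timer is a Blueprint that drives a countdown shown through the player's HUD.
; On Tick it accumulates delta time, and once more than a second passes it resets the accumulator to zero, dropping any overshoot.
; It then casts the first player controller's HUD to BP_HUD and decrements its TimeAmount by one, with no lower limit in this graph.
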(event EventTick
  (params (DeltaSeconds :type Float%20%28single-precision%29))
  (Variables|Default|SetbuildingTime (+ DeltaSeconds (Variables|Default|GetbuildingTime)))
  (if (> (Variables|Default|GetbuildingTime) 1.0)
    (Variables|Default|SetbuildingTime 0.0)
    (bind _asbp_hud_c (Utilities|Casting|CastToBP_HUD (HUD|GetHUD (Game|GetPlayerController 0))))
    (Variables|/Game/Assets/BP_HUD.BP_HUD_C|SetTimeAmount _asbp_hud_c (- (Variables|/Game/Assets/BP_HUD.BP_HUD_C|GetTimeAmount _asbp_hud_c) 1))))

(fn ConstructionScript)