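; BP_Menu_HUD is the title screen HUD, drawing the start prompt and control help over a full-screen title texture.
; Everything is drawn immediate-mode in DrawHUD, positioned with fixed pixel offsets from the screen size.
; The control lines start at X equal to the screen width, placing them past the right edge.
; It only draws, with no handling of the Enter key it advertises.
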(event EventDrawHUD
  (params (SizeX :type Integer) (SizeY :type Integer))
  (Canvas|DrawTexture "/Game/Assets/T_Title_Screen.T_Title_Screen" 0.0 0.0 (Math|Conversions|ToFloat(Integer) SizeX) (Math|Conversions|ToFloat(Integer) SizeY) 0.0 0.0 1.0 1.0 "(R=1.000000,G=1.000000,B=1.000000,A=1.000000)")
  (HUD|DrawText "Press enter to start" "(R=1.000000,G=1.000000,B=1.000000,A=1.000000)" (- (/ (Math|Conversions|ToFloat(Integer) SizeX) 2.0) 2.5e+02) (/ (Math|Conversions|ToFloat(Integer) SizeY) 2.0) 0 5.0 false)
  (HUD|DrawText "Controls" "(R=1.000000,G=1.000000,B=1.000000,A=1.000000)" (Math|Conversions|ToFloat(Integer) SizeX) (- (Math|Conversions|ToFloat(Integer) SizeY) 3e+02) 0 2.0 false)
  (HUD|DrawText "WASD: Move, Space: Switch between hover and flight mode" "(R=1.000000,G=1.000000,B=1.000000,A=1.000000)" (Math|Conversions|ToFloat(Integer) SizeX) (- (Math|Conversions|ToFloat(Integer) SizeY) 3e+02) 0 1.0 false)
  (HUD|DrawText "Left-Click: Regular Shot, Right-Click (Hover Mode): Homing Shots, Right-Click (Boost Mode): Carpet Bomb" "(R=1.000000,G=1.000000,B=1.000000,A=1.000000)" (Math|Conversions|ToFloat(Integer) SizeX) (- (Math|Conversions|ToFloat(Integer) SizeY) 1e+02) 0 1.0 false))

(fn ConstructionScript
  (|CallParentFunction))